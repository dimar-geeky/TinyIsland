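; SeaBP is an actor that lays out a grid of instanced static meshes, presumably forming a sea surface.
; The Construction Script halves the row and column counts to roughly center the grid on the actor, then adds one instance per cell in nested loops.
; InstanceScale sets both instance size and spacing, based on a 100-unit cell.
; The event graph holds only disabled placeholder events, so nothing runs during play.
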(fn `UserConstructionScript`
  (locals (rowStartShift :type Integer :default 0) (colStartShift :type Integer :default 0))
  (bind _instancescale (`self.instanceScale`))
  (`|ExecutionSequence`
    (:`then_0`
      (set `local.rowStartShift` (/ (`self.rowsNum`) 2))
      (set `local.colStartShift` (/ (`self.colsNum`) 2)))
    (:`then_1`
      (for _index (range (`self.colsNum`))
        (for _index_2 (range (`self.rowsNum`))
          (`InstancedStaticMeshComponent.AddInstance` (`self.InstancedStaticMesh`) (`KismetMathLibrary.MakeTransform` (`KismetMathLibrary.MakeVector` (* (* (- _index (`local.colStartShift`)) 100) _instancescale) (* (* (- _index_2 (`local.rowStartShift`)) 100) _instancescale)) (struct) (`KismetMathLibrary.Conv_DoubleToVector` (`self.instanceScale`)))))))))